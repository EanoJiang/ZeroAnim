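; BP_HuanGui_PlumPole is a HuanGui character Blueprint in the PlumPoleTest folder that assembles a multi-part skeletal body, with no gameplay logic of its own.
; After running the parent construction script, it makes head and lashes follow the body's pose through Leader Pose.
; Tick prerequisites order updates from the main Mesh to the body, then to cloth and hair, so those parts evaluate after the body each frame.
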(event EventBeginPlay)

(event Collision|EventActorBeginOverlap
  (params (OtherActor :type Actor%20Object%20Reference)))

(event EventTick
  (params (DeltaSeconds :type Float%20%28single-precision%29)))

(fn ConstructionScript
  (bind _huangui_body (Variables|Default|GetHuanGui_Body))
  (|CallParentFunction)
  (Components|SkinnedMesh|SetLeaderPoseComponent (Variables|Default|GetHuanGui_Head) _huangui_body true false)
  (Components|SkinnedMesh|SetLeaderPoseComponent (Variables|Default|GetHuanGui_Lashes) _huangui_body true false)
  (Class|ActorComponent|AddTickPrerequisiteComponent _huangui_body (Variables|Character|GetMesh))
  (Class|ActorComponent|AddTickPrerequisiteComponent (Variables|Default|GetHuanGui_Cloth01) _huangui_body)
  (Class|ActorComponent|AddTickPrerequisiteComponent (Variables|Default|GetHuanGui_Cloth02) _huangui_body)
  (Class|ActorComponent|AddTickPrerequisiteComponent (Variables|Default|GetHuanGui_Hair01) _huangui_body)
  (Class|ActorComponent|AddTickPrerequisiteComponent (Variables|Default|GetHuanGui_Hair02) _huangui_body))