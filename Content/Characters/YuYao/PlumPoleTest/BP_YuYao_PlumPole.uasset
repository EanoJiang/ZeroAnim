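; BP_YuYao_PlumPole is a YuYao character Blueprint variant in the PlumPoleTest folder, assembling a multi-part skeletal character.
; Its construction script runs the parent's, then makes the head follow the body's pose via Leader Pose Component.
; Tick prerequisites order the body after the main Mesh, and the two cloth parts and hair after the body.
; The event graph holds only disabled placeholder events.
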(event EventBeginPlay)

(event Collision|EventActorBeginOverlap
  (params (OtherActor :type Actor%20Object%20Reference)))

(event EventTick
  (params (DeltaSeconds :type Float%20%28single-precision%29)))

(fn ConstructionScript
  (bind _yuu_body (Variables|Default|GetYuu_Body))
  (|CallParentFunction)
  (Components|SkinnedMesh|SetLeaderPoseComponent (Variables|Default|GetYuu_Head) _yuu_body true false)
  (Class|ActorComponent|AddTickPrerequisiteComponent _yuu_body (Variables|Character|GetMesh))
  (Class|ActorComponent|AddTickPrerequisiteComponent (Variables|Default|GetYuu_Cloth01) _yuu_body)
  (Class|ActorComponent|AddTickPrerequisiteComponent (Variables|Default|GetYuu_Cloth02) _yuu_body)
  (Class|ActorComponent|AddTickPrerequisiteComponent (Variables|Default|GetYuu_Hair01) _yuu_body))